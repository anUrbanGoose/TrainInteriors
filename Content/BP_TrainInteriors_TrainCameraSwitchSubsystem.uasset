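; Train Interiors subsystem that tracks whether the first-person train camera is active.
; On begin play it enables player 0 input and caches the First Person Vehicles camera switch subsystem, if present.
; The perspective toggle input flips the flag when the controlled pawn's locomotive interior mixin reports first person in use, then notifies that subsystem.
; FirstPersonVehiclesSwitched copies that subsystem's state back, syncing both mods.
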(event `self.ReceiveBeginPlay`
  (bind _returnvalue (`GameplayStatics.GetPlayerController` 0))
  (bind _returnvalue_2 (`SubsystemActorManager.K2_GetSubsystemActor` (subsystem `SubsystemActorManager`) "/FirstPersonVehicles/BP_FirstPersonVehicles_VehicleCameraSwitchSubsystem.BP_FirstPersonVehicles_VehicleCameraSwitchSubsystem_C"))
  (`self.EnableInput` _returnvalue)
  (`BlueprintLoggingLibrary.LogDisplay` (`KismetStringLibrary.JoinStringArray` (`|MakeArray` "Train Interiors - Enabled input for controller:" (`KismetSystemLibrary.GetDisplayName` _returnvalue))))
  (`/Engine/EditorBlueprintResources/StandardMacros.IsValid` _returnvalue_2
    (:`Is Valid`
      (set `self.FirstPersonVehiclesSubsystem` _returnvalue_2))))

(event `EnhancedInput|/TrainInteriors/Input/IA_TrainInteriors_PerspectiveToggle`
  (params (ActionValue :type Boolean) (ElapsedSeconds :type "Float (double-precision)") (TriggeredSeconds :type "Float (double-precision)") (InputAction :type "InputAction Object Reference" :default "/TrainInteriors/Input/IA_TrainInteriors_PerspectiveToggle.IA_TrainInteriors_PerspectiveToggle"))
  (bind _firstpersonvehiclessubsystem (`self.FirstPersonVehiclesSubsystem`))
  (:`Started`
    (if (`/TrainInteriors/Locomotive_Interior_Mixin.LocomotiveIsUsingFirstPerson` (`BlueprintActorMixin.GetActorMixin` (`Controller.K2_GetPawn` (`GameplayStatics.GetPlayerController` 0)) "/TrainInteriors/Locomotive_Interior_Mixin.Locomotive_Interior_Mixin_C"))
      (bind _output_get (set `self.TrainFirstPersonActive` (not (`self.TrainFirstPersonActive`))))
      (`BlueprintLoggingLibrary.LogDisplay` (`KismetStringLibrary.JoinStringArray` (`|MakeArray` "Train First Person Camera active:" (`KismetStringLibrary.Conv_BoolToString` _output_get))))
      (if (`KismetSystemLibrary.IsValid` _firstpersonvehiclessubsystem)
        (`/FirstPersonVehicles/BP_FirstPersonVehicles_VehicleCameraSwitchSubsystem.TrainInteriorCameraSwitched` _firstpersonvehiclessubsystem)))))

(event `FirstPersonVehiclesSwitched`
  (bind _output_get (set `self.TrainFirstPersonActive` (`/FirstPersonVehicles/BP_FirstPersonVehicles_VehicleCameraSwitchSubsystem.VehicleFirstPersonActive` (`self.FirstPersonVehiclesSubsystem`))))
  (`BlueprintLoggingLibrary.LogDisplay` (`KismetStringLibrary.JoinStringArray` (`|MakeArray` "Train First Person Camera active:" (`KismetStringLibrary.Conv_BoolToString` _output_get)))))

(fn `UserConstructionScript`)